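; Static LOD ocean actor that keeps its OceanPreLod2 component facing the player camera.
; Each Tick builds a rotation from the vector between the component and the camera with MakeRotFromZ, aiming the component's Z axis at the camera like a billboard.
; An alternative look-at local rotation of the actor is left unconnected and never runs.
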(event EventBeginPlay)

(event Collision|EventActorBeginOverlap
  (params (OtherActor :type Actor%20Object%20Reference)))

(event EventTick
  (params (DeltaSeconds :type Float%20%28single-precision%29))
  (bind _oceanprelod2 (Variables|Default|GetOceanPreLod2))
  (Transformation|SetWorldRotation _oceanprelod2 (Math|Rotator|MakeRotfromZ (- (Camera|GetCameraLocation (Game|GetPlayerCameraManager 0)) (Transformation|GetWorldLocation _oceanprelod2))) false false))

(fn ConstructionScript)